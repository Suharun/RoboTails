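; Camera actor that takes over the first player controller's view on BeginPlay and follows the Player in the Y-Z plane, as in a side-scroller.
; Each Tick, GetNewY and GetNewZ move the camera only when the Player leaves a dead zone around it, trailing at that zone's edge.
; LimitY and LimitZ then clamp the result between MinPosition and MaxPosition before the actor moves, with X fixed at XOffset.
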(event EventBeginPlay
  (Game|Player|SetViewTargetwithBlend (Game|GetPlayerController 0) self 0.0 "VTBlend_Linear" 0.0 false))

(event Collision|EventActorBeginOverlap
  (params (OtherActor :type Actor%20Object%20Reference)))

(event EventTick
  (params (DeltaSeconds :type Float%20%28single-precision%29))
  (bind _new_y (CallFunction|GetNewY))
  (Variables|Default|SetCameraY _new_y)
  (bind _new_z (CallFunction|GetNewZ))
  (Variables|Default|SetCameraZ _new_z)
  (CallFunction|LimitY)
  (CallFunction|LimitZ)
  (Transformation|SetActorLocation (Math|Vector|MakeVector (Variables|Default|GetX%20Offset) (Variables|Default|GetCameraY) (Variables|Default|GetCameraZ)) false false))

(fn ConstructionScript)

(fn GetNewY
  (bind _player (Variables|Default|GetPlayer))
  (bind _player_2 (Variables|Default|GetPlayer))
  (bind _y_deadzone (Variables|Default|GetY%20DeadZone))
  (bind _y_deadzone_2 (Variables|Default|GetY%20DeadZone))
  (bind _returnvalue (Transformation|GetActorLocation _player_2))
  (bind _returnvalue_2 (Transformation|GetActorLocation _player))
  (bind _returnvalue_3 (- (.y _returnvalue) _y_deadzone))
  (bind _returnvalue_4 (+ (.y _returnvalue_2) _y_deadzone_2))
  (if (> _returnvalue_3 (.y (Transformation|GetActorLocation)))
    (return _returnvalue_3)
    (elif (< _returnvalue_4 (.y (Transformation|GetActorLocation)))
      (return _returnvalue_4)
      (else
        (return (Variables|Default|GetCameraY))))))

(fn GetNewZ
  (bind _player (Variables|Default|GetPlayer))
  (bind _z_deadzone (Variables|Default|GetZ%20DeadZone))
  (bind _player_2 (Variables|Default|GetPlayer))
  (bind _z_deadzone_2 (Variables|Default|GetZ%20DeadZone))
  (bind _returnvalue (Transformation|GetActorLocation _player_2))
  (bind _returnvalue_2 (Transformation|GetActorLocation _player))
  (bind _returnvalue_3 (- (.z _returnvalue) _z_deadzone_2))
  (bind _returnvalue_4 (+ (.z _returnvalue_2) _z_deadzone))
  (if (> _returnvalue_3 (.z (Transformation|GetActorLocation)))
    (return _returnvalue_3)
    (elif (< _returnvalue_4 (.z (Transformation|GetActorLocation)))
      (return _returnvalue_4)
      (else
        (return (Variables|Default|GetCameraZ))))))

(fn LimitY
  (bind _maxposition (Variables|Default|GetMaxPosition))
  (bind _minposition (Variables|Default|GetMinPosition))
  (if (> (Variables|Default|GetCameraY) (.y _maxposition))
    (Variables|Default|SetCameraY (.y _maxposition))
    (elif (< (Variables|Default|GetCameraY) (.y _minposition))
      (Variables|Default|SetCameraY (.y _minposition))))
  (return))

(fn LimitZ
  (bind _maxposition (Variables|Default|GetMaxPosition))
  (bind _minposition (Variables|Default|GetMinPosition))
  (if (> (Variables|Default|GetCameraZ) (.z _maxposition))
    (Variables|Default|SetCameraZ (.z _maxposition))
    (elif (< (Variables|Default|GetCameraZ) (.z _minposition))
      (Variables|Default|SetCameraZ (.z _minposition))))
  (return))