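; Key pickup that bobs up and down and turns out the lights when the player collects it.
; Tick drives a timeline through DoOnce and FlipFlop, alternating forward and reverse playback to nudge the actor's height.
; On box overlap, it shows a dialogue hint if no LightBalb actors exist, plays sound and particle effects, destroys itself and calls LightsOut on the player.
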(event OnComponentBeginOverlap(Box)
  (params (OverlappedComponent :type Primitive%20Component%20Object%20Reference) (OtherActor :type Actor%20Object%20Reference) (OtherComp :type Primitive%20Component%20Object%20Reference) (OtherBodyIndex :type Integer) (bFromSweep :type Boolean) (SweepResult :type Hit%20Result%20Structure%20%28by%20ref%29))
  (bind _asplayer (Utilities|Casting|CastToPlayer OtherActor))
  (bind _outactors (Actor|GetAllActorsOfClass "/Game/BluePrints/LightBalb.LightBalb_C"))
  (if (Utilities|Array|IsValidIndex _outactors)
    _
    (else
      (Default|CreateDialogue _asplayer "Drat, I can't see anything. 
I need to leave a trail behind." 0 3.0)))
  (CallFunction|CollectItem)
  (Default|LightsOut _asplayer))

(event Custom|CollectItem
  (Audio|PlaySound2D 0 1.0 1.0 0.0 0 0)
  (Effects|SpawnEmitteratLocation 0 "0, 0, 0")
  (Actor|DestroyActor))

(event EventBeginPlay)

(event Collision|EventActorBeginOverlap
  (params (OtherActor :type Actor%20Object%20Reference)))

(event EventTick
  (params (DeltaSeconds :type Float%20%28single-precision%29))
  (bind _returnvalue (Transformation|GetActorLocation))
  (Utilities|FlowControl|DoOnce false :!label _label
    (:Completed
      (Utilities|FlowControl|FlipFlop
        (:A
          (bind _newtrack_0 (Timeline|BobbingTimeLiNE PlayFromStart)
            (:Update
              (Transformation|SetActorLocation (Math|Vector|MakeVector (.x _returnvalue) (.y _returnvalue) (+ (.z _returnvalue) (Math|Float|Lerp -1.0 1.0 _newtrack_0))) false false))
            (:Finished
              (goto _label Reset))))
        (:B
          (Timeline|BobbingTimeLiNE ReverseFromEnd))))))

(fn ConstructionScript)