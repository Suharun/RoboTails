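; A 2D lock actor that opens and stops blocking once its referenced Key actor no longer exists.
; Tick polls the validity of Key and keeps IsOpen in sync with it.
; When Key is invalid, a DoOnce plays the opening flipbook, switches to the open flipbook after a short delay, then disables the Box collision.
; An alternative IsActorBeingDestroyed check is left unconnected.
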(event EventBeginPlay)

(event Collision|EventActorBeginOverlap
  (params (OtherActor :type Actor%20Object%20Reference)))

(event EventTick
  (params (DeltaSeconds :type Float%20%28single-precision%29))
  (Utilities|IsValid (Variables|Default|GetKey)
    (:Is%20Valid
      (Variables|Default|SetIsOpen false))
    (:Is%20Not%20Valid
      (Variables|Default|SetIsOpen true)
      (Utilities|FlowControl|DoOnce false
        (:Completed
          (Sprite|SetFlipbook (Variables|Default|GetPaperFlipbook) "/Game/Animations/OpeningLock.OpeningLock")
          (Utilities|FlowControl|Delay 0.2)
          (Sprite|SetFlipbook (Variables|Default|GetPaperFlipbook) "/Game/Animations/OpenLock.OpenLock")
          (Collision|SetCollisionEnabled (Variables|Default|GetBox) "NoCollision"))))))

(fn ConstructionScript)