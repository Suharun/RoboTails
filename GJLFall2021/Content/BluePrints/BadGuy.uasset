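; BadGuy is a flipbook villain that appears and taunts the player in a scripted trap cutscene, then destroys the level's Key actor.
; When the player's DialogueTrigger is set, Tick teleports it into place with a spawn animation and polls player story flags to advance the dialogue.
; Nested booleans and DoOnce nodes sequence the lines, each shown temporarily through a DialogueIU widget created by CinematicDialogue.
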(event Custom|Dialogue
  (bind _player (Variables|Default|GetPlayer))
  (bind _widget (Variables|Default|GetWidget))
  (bind _widget_2 (Variables|Default|GetWidget))
  (bind _widget_3 (Variables|Default|GetWidget))
  (bind _widget_4 (Variables|Default|GetWidget))
  (bind _key (Variables|Default|GetKey))
  (bind _widget_5 (Variables|Default|GetWidget))
  (if (Variables|Default|GetGreetings)
    (if (Variables|/Game/BluePrints/Player.Player_C|GetGreeting _player)
      (if (Variables|Default|GetAbandoned)
        (if (Variables|/Game/BluePrints/Player.Player_C|GetRobotsFlee _player)
          (if (Variables|Default|GetFear)
            (if (Variables|/Game/BluePrints/Player.Player_C|GetCurses _player)
              (if (Variables|Default|GetBoast)
                (if (Variables|Default|GetEvil%20Trap%20Thing)
                  (Utilities|IsValid _key
                    (:Is%20Valid
                      (Utilities|FlowControl|Delay 5.0)
                      (Actor|DestroyActor _key)))
                  (else
                    (Utilities|FlowControl|DoOnce false
                      (:Completed
                        (Utilities|FlowControl|Delay 1.0)
                        (CallFunction|CinematicDialogue)
                        (Utilities|FlowControl|Delay 4.0)
                        (Rendering|SetVisibility _widget false false)
                        (UserInterface|SetWidget _widget 0)
                        (Variables|Default|SetEvil%20Trap%20Thing true)))))
                (else
                  (Utilities|FlowControl|DoOnce false
                    (:Completed
                      (Utilities|FlowControl|Delay 1.0)
                      (CallFunction|CinematicDialogue)
                      (Utilities|FlowControl|Delay 5.0)
                      (Rendering|SetVisibility _widget_5 false false)
                      (UserInterface|SetWidget _widget_5 0)
                      (Variables|Default|SetBoast true)
                      (Math|Integer|IncrementInt (Variables|Default|GetStringIndex)))))))
            (else
              (Utilities|FlowControl|DoOnce false
                (:Completed
                  (Utilities|FlowControl|Delay 1.0)
                  (CallFunction|CinematicDialogue)
                  (Utilities|FlowControl|Delay 2.0)
                  (Rendering|SetVisibility _widget_4 false false)
                  (UserInterface|SetWidget _widget_4 0)
                  (Variables|Default|SetFear true))))))
        (else
          (Utilities|FlowControl|DoOnce false
            (:Completed
              (Utilities|FlowControl|Delay 1.0)
              (CallFunction|CinematicDialogue)
              (Utilities|FlowControl|Delay 5.0)
              (Rendering|SetVisibility _widget_3 false false)
              (UserInterface|SetWidget _widget_3 0)
              (Variables|Default|SetAbandoned true))))))
    (else
      (Utilities|FlowControl|DoOnce false
        (:Completed
          (Utilities|FlowControl|Delay 1.0)
          (CallFunction|CinematicDialogue)
          (Utilities|FlowControl|Delay 2.0)
          (Rendering|SetVisibility _widget_2 false false)
          (UserInterface|SetWidget _widget_2 0)
          (Variables|Default|SetGreetings true))))))

(event Custom|Check%20Next%20Dialogue
  (bind _player (Variables|Default|GetPlayer))
  (if (Variables|/Game/BluePrints/Player.Player_C|GetScream _player)
    (Utilities|FlowControl|DoOnce false)
    (elif (Variables|/Game/BluePrints/Player.Player_C|GetCurses _player)
      (Utilities|FlowControl|DoOnce false
        (:Completed
          (Math|Integer|IncrementInt (Variables|Default|GetStringIndex))))
      (elif (Variables|/Game/BluePrints/Player.Player_C|GetRobotsFlee _player)
        (Utilities|FlowControl|DoOnce false
          (:Completed
            (Math|Integer|IncrementInt (Variables|Default|GetStringIndex))))
        (elif (Variables|/Game/BluePrints/Player.Player_C|GetGreeting _player)
          (Utilities|FlowControl|DoOnce false
            (:Completed
              (Math|Integer|IncrementInt (Variables|Default|GetStringIndex)))))))))

(event EventBeginPlay
  (Variables|Default|SetStringArray (Utilities|Array|MakeArray "HAHAHAHA 
I have trapped you  
once again R0B1N" "It looks like your little, 
\"friends\" are going to abandon you." "SCRAM!" "Of course I did!  
I AM ALL KNOWING" "AND NOW.... 
ITS TIME FOR YOU TO ROT IN THIS PIT! 
GOODBYE"))
  (bind _outactors (Actor|GetAllActorsOfClass "/Game/BluePrints/Key.Key_C"))
  (Variables|Default|SetKey (Utilities|Array|Get(acopy) _outactors)))

(event Collision|EventActorBeginOverlap
  (params (OtherActor :type Actor%20Object%20Reference)))

(event EventTick
  (params (DeltaSeconds :type Float%20%28single-precision%29))
  (Sprite|SetFlipbook (Variables|Default|GetPaperFlipbook) (Utilities|Select :Index (Variables|Default|GetState) :Option%200 "/Game/Animations/Idle.Idle" :Option%201 "/Game/Assets/EnemyBoss/Spawn.Spawn"))
  (if (Variables|/Game/BluePrints/Player.Player_C|GetDialogueTrigger (Variables|Default|GetPlayer))
    (Utilities|FlowControl|Sequence
      (:then_0
        (Utilities|FlowControl|DoOnce false
          (:Completed
            (Transformation|SetActorLocation "-200.000000,2393.000000,-2936.000000" false false)
            (Variables|Default|SetState 1)
            (Utilities|FlowControl|Delay 2.0)
            (Variables|Default|SetState 0))))
      (:then_1
        (CallFunction|CheckNextDialogue))
      (:then_2
        (CallFunction|Dialogue)))))

(fn ConstructionScript)

(fn StateMachine)

(fn CinematicDialogue
  (Rendering|SetVisibility (Variables|Default|GetWidget) true false)
  (bind _returnvalue (UserInterface|CreateWidget "/Game/UI/DialogueIU.DialogueIU_C" (Game|GetPlayerController 0)))
  (Variables|/Game/UI/DialogueIU.DialogueIU_C|SetMessage _returnvalue (Utilities|Array|Get(acopy) (Variables|Default|GetStringArray) (Variables|Default|GetStringIndex)))
  (Class|Border|SetBrushColor (Variables|/Game/UI/DialogueIU.DialogueIU_C|GetBorder_0 _returnvalue) "(R=0.717014,G=0.464316,B=0.489554,A=1.000000)")
  (UserInterface|SetWidget (Variables|Default|GetWidget) _returnvalue))