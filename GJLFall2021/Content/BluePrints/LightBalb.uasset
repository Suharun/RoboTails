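; LightBalb is a sprite robot actor that takes its tint from its State on BeginPlay.
; In cinematic mode, Tick steps it along Y by fixed, frame-dependent offsets: backward and rotated while the Player's Villain has Fear, otherwise forward up to MaxY while the Player moves.
; Outside cinematics it destroys itself after falling below a Z threshold.
; The RobotDetection overlap only casts to LightBalb, with no further action.
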(event OnComponentBeginOverlap(RobotDetection)
  (params (OverlappedComponent :type Primitive%20Component%20Object%20Reference) (OtherActor :type Actor%20Object%20Reference) (OtherComp :type Primitive%20Component%20Object%20Reference) (OtherBodyIndex :type Integer) (bFromSweep :type Boolean) (SweepResult :type Hit%20Result%20Structure%20%28by%20ref%29))
  (Utilities|Casting|CastToLightBalb OtherActor))

(event EventBeginPlay
  (Sprite|SetSpriteColor (Variables|Default|GetRobot) (Utilities|Select :Index (Variables|Default|Getstate) :NewEnumerator0 "(R=1.000000,G=1.000000,B=1.000000,A=1.000000)" :NewEnumerator1 "(R=0.000000,G=0.185913,B=0.826389,A=1.000000)" :NewEnumerator2 "(R=1.000000,G=0.966577,B=0.000000,A=1.000000)")))

(event Collision|EventActorBeginOverlap
  (params (OtherActor :type Actor%20Object%20Reference)))

(event EventTick
  (params (DeltaSeconds :type Float%20%28single-precision%29))
  (bind _returnvalue (Transformation|GetActorLocation))
  (bind _returnvalue_2 (Transformation|GetActorLocation))
  (bind _returnvalue_3 (Transformation|GetActorLocation))
  (bind _maxy (Variables|Default|GetMaxY))
  (if (Variables|Default|GetbIsCinematic)
    (if (Variables|/Game/BluePrints/BadGuy.BadGuy_C|GetFear (Variables|/Game/BluePrints/Player.Player_C|GetVillain (Variables|Default|GetPlayer)))
      (Transformation|SetActorLocation (Math|Vector|MakeVector (.x _returnvalue_2) (+ (.y _returnvalue_2) -9.0) (.z _returnvalue_2)) false false)
      (Transformation|SetActorRotation "0,270.000000, 0")
      (elif (Variables|/Game/BluePrints/Player.Player_C|Getis%20Moving (Variables|Default|GetPlayer))
        (Transformation|SetActorLocation (Math|Vector|MakeVector (.x _returnvalue_3) (+ (.y _returnvalue_3) 9.0) (.z _returnvalue_3)) false false)
        (if (>= (.y _returnvalue) _maxy)
          (Transformation|SetActorLocation (Math|Vector|MakeVector (.x _returnvalue) _maxy (.z _returnvalue)) false false))))
    (elif (<= (.z (Transformation|GetActorLocation)) -4e+03)
      (Actor|DestroyActor))))

(fn ConstructionScript)